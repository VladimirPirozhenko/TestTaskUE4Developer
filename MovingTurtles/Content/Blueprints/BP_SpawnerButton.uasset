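; Spawner button actor that spawns a turtle from a nest when pressed.
; On BeginPlay it calls OnInteracted, then binds a handler to the OnSpawnerButtonPressed dispatcher.
; The handler tells BPNest to spawn a turtle, plays a blip at the button and runs a one-shot push animation on ButtonMesh.
; After a short delay it returns the mesh to Animation Blueprint mode.
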(event Custom|OnSpawnerButtonPressed_Event_0
  (Class|Nest|SpawnTurtle (Variables|Nest|GetBP_Nest))
  (Audio|PlaySoundatLocation "/Game/Sounds/blip1.blip1" (Transformation|GetActorLocation self) "0, 0, 0" 1.0 1.0 0.0 0 0 0)
  (Components|Animation|PlayAnimation (Variables|Default|GetButtonMesh) "/Game/scifi-button/source/button_Anim_push_001.button_Anim_push_001" false)
  (Utilities|FlowControl|Delay 0.75)
  (Components|Animation|SetAnimationMode (Variables|Default|GetButtonMesh) "AnimationBlueprint"))

(event EventBeginPlay
  (Class|SpawnerButton|OnInteracted)
  (EventDispatchers|AssignOnSpawnerButtonPressed (delegate Custom|OnSpawnerButtonPressed_Event_0)))

(event Collision|EventActorBeginOverlap
  (params (OtherActor :type Actor%20Object%20Reference)))

(event EventTick
  (params (DeltaSeconds :type Float%20%28single-precision%29)))

(fn ConstructionScript)