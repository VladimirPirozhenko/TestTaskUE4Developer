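; Movement strategy Blueprint that moves an actor toward a destination in a stop-and-go rhythm.
; Each Tick runs MoveToDestination, which steps the location at constant speed, turns the actor toward the target and flags arrival.
; Chained Delays on Tick toggle IsStopped, zeroing speed for short pauses between moves; Stop sets the same flag.
; On arrival, movement ends and a DoOnce fires OnMovementOver.
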(event EventBeginPlay)

(event EventTick
  (params (DeltaSeconds :type Float%20%28single-precision%29))
  (Utilities|FlowControl|Sequence
    (:then_0
      (if (Variables|Default|GetIsMovementOver)
        (Utilities|FlowControl|DoOnce false
          (:Completed
            (Default|CallOnMovementOver)))
        (else
          (CallFunction|MovetoDestination (stale EventMovetoDestination Destination) DeltaSeconds (stale EventMovetoDestination Speed) (stale EventMovetoDestination Actor)))))
    (:then_1
      (if (not (Variables|Default|GetIsStopped))
        (Utilities|FlowControl|Delay 1.0)
        (Variables|Default|SetIsStopped true)
        (Utilities|FlowControl|Delay 0.5)
        (Variables|Default|SetIsStopped false)))))

(event EventMovetoDestination
  (params (Actor :type Actor%20Object%20Reference) (Destination :type Vector :default "0, 0, 0") (Speed :type Float%20%28single-precision%29))
  (CallFunction|MovetoDestination Destination (stale EventTick DeltaSeconds) Speed Actor))

(fn MovetoDestination
  (params (Destination :type Vector) (DeltaTime :type Float%20%28single-precision%29) (InterpSpeed :type Float%20%28single-precision%29) (Actor :type Actor%20Object%20Reference))
  (if (Variables|Default|GetIsStopped)
    (LocalVariables|SetSpeed 0.0)
    (else
      (LocalVariables|SetSpeed InterpSpeed)))
  (Transformation|SetActorLocation Actor (Math|Interpolation|VInterptoConstant (Transformation|GetActorLocation Actor) Destination DeltaTime (LocalVariables|GetSpeed)) false false)
  (Transformation|SetActorRotation Actor (Math|Rotator|FindLookatRotation (Transformation|GetActorLocation Actor) Destination))
  (if (Math|Vector|VectorIsNearlyZero (- (Transformation|GetActorLocation Actor) Destination) 0.0005)
    (Variables|Default|SetIsMovementOver true)))

(fn Stop
  (Variables|Default|SetIsStopped true))