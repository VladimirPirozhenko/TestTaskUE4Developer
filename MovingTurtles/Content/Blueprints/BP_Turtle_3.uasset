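; BP_Turtle_3 is an animated turtle actor that moves via a BPBackAndForthMovementStrategy component and celebrates when that movement ends.
; On BeginPlay it loops a shark skeleton animation, spawns a large explosion, attaches fire to the mesh and starts a swimming sound.
; The component's OnMovementOver event triggers PlayWinningSound, which plays a victory cheer and smoke, stops the animation and swimming sound, and destroys the fire.
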(event Custom|PlayWinningSound
  (bind _returnvalue (Transformation|GetActorLocation))
  ;[1 1 1] Destination reached
  (Audio|PlaySoundatLocation "/Game/Sounds/mixkit-male-voice-cheer-victory-2011.mixkit-male-voice-cheer-victory-2011" _returnvalue "0, 0, 0" 1.0 1.0 0.0 0 0 0)
  (Audio|Components|Audio|Stop (Variables|Default|GetTutleMesh))
  (Audio|Components|Audio|Stop (Variables|Default|GetMovingSound))
  (Effects|SpawnEmitteratLocation "/Game/Common/StarterContent/Particles/P_Smoke.P_Smoke" _returnvalue)
  (Components|DestroyComponent (stale EventBeginPlay _returnvalue)))

(event EventBeginPlay
  (Components|Animation|PlayAnimation (Variables|Default|GetTutleMesh) "/Game/sport-shark-animated-free-download/source/Sport_Shark_Skeleton_Sequence.Sport_Shark_Skeleton_Sequence" true)
  (Effects|SpawnEmitteratLocation "/Game/Common/StarterContent/Particles/P_Explosion.P_Explosion" (Transformation|GetActorLocation) "0, 0, 0" "10.000000,10.000000,10.000000")
  (bind _returnvalue (Effects|SpawnEmitterAttached "/Game/Common/StarterContent/Particles/P_Fire.P_Fire" (Variables|Default|GetTutleMesh) "None"))
  (EventDispatchers|BindEventtoOnMovementOver (Variables|Default|GetBP_BackAndForthMovementStrategy) (delegate Custom|PlayWinningSound))
  (bind _returnvalue_2 (Audio|SpawnSoundatLocation "/Game/Sounds/mixkit-sea-swimming-loop-1181.mixkit-sea-swimming-loop-1181" (Transformation|GetActorLocation) "0, 0, 0" 1.0 1.0 0.0 0 0))
  (Variables|Default|SetMovingSound _returnvalue_2))

(fn ConstructionScript)