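; Standard movement strategy Blueprint that moves a given actor in a straight line to a destination.
; Tick and the MovetoDestination event feed MoveToDestination, which steps the location with VInterpToConstant without sweep and turns the actor toward the target.
; Near-zero remaining distance sets IsMovementOver, after which Tick fires CallOnMovementOver through a DoOnce that is never reset.
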(event EventBeginPlay)

(event EventTick
  (params (DeltaSeconds :type Float%20%28single-precision%29))
  (if (Variables|Default|GetIsMovementOver)
    (Utilities|FlowControl|DoOnce false
      (:Completed
        (Default|CallOnMovementOver)))
    (else
      (CallFunction|MovetoDestination (stale EventMovetoDestination Destination) DeltaSeconds (stale EventMovetoDestination Speed) (stale EventMovetoDestination Actor)))))

(event EventMovetoDestination
  (params (Actor :type Actor%20Object%20Reference) (Destination :type Vector :default "0, 0, 0") (Speed :type Float%20%28single-precision%29))
  (CallFunction|MovetoDestination Destination (stale EventTick DeltaSeconds) Speed Actor))

(fn MovetoDestination
  (params (Destination :type Vector) (DeltaTime :type Float%20%28single-precision%29) (InterpSpeed :type Float%20%28single-precision%29) (TargetActor :type Actor%20Object%20Reference))
  (bind _returnvalue (Transformation|GetActorLocation TargetActor))
  (Transformation|SetActorLocation TargetActor (Math|Interpolation|VInterptoConstant _returnvalue Destination DeltaTime InterpSpeed) false false)
  (Transformation|SetActorRotation TargetActor (Math|Rotator|FindLookatRotation _returnvalue Destination))
  (if (Math|Vector|VectorIsNearlyZero (- (Transformation|GetActorLocation TargetActor) Destination) 0.0005)
    (Variables|Default|SetIsMovementOver true)))