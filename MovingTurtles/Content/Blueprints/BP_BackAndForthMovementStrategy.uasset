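; Movement strategy that moves a given actor toward a destination in a back-and-forth pattern, facing along the path from its start.
; Tick interpolates the actor at constant speed, while chained delays flip IsForthMovement to alternate longer advances with shorter retreats toward the recorded initial position.
; Reaching the destination sets IsMovementOver and calls OnMovementOver once; Stop sets the retreat flag.
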(event EventBeginPlay)

(event EventTick
  (params (DeltaSeconds :type Float%20%28single-precision%29))
  (Utilities|FlowControl|Sequence
    (:then_0
      (if (Variables|Default|GetIsMovementOver)
        (Utilities|FlowControl|DoOnce false
          (:Completed
            (Default|CallOnMovementOver)))
        (else
          (CallFunction|MovetoDestination (stale EventMovetoDestination Destination) DeltaSeconds (stale EventMovetoDestination Speed) (stale EventMovetoDestination Actor)))))
    (:then_1
      (if (not (Variables|Default|GetIsForthMovement))
        (Utilities|FlowControl|Delay 1.0)
        (Variables|Default|SetIsForthMovement true)
        (Utilities|FlowControl|Delay 0.5)
        (Variables|Default|SetIsForthMovement false)))))

(event EventMovetoDestination
  (params (Actor :type Actor%20Object%20Reference) (Destination :type Vector :default "0, 0, 0") (Speed :type Float%20%28single-precision%29))
  (Utilities|FlowControl|Sequence
    (:then_0
      (Variables|Default|SetInitialPosition (Transformation|GetActorLocation Actor)))
    (:then_1
      (if (Variables|Default|GetIsMovementOver)
        (Utilities|FlowControl|DoOnce false
          (:Completed
            (Default|CallOnMovementOver)))
        (else
          (CallFunction|MovetoDestination Destination (stale EventTick DeltaSeconds) Speed Actor))))))

(fn MovetoDestination
  (params (Destination :type Vector) (DeltaTime :type Float%20%28single-precision%29) (InterpSpeed :type Float%20%28single-precision%29) (Actor :type Actor%20Object%20Reference))
  (bind _initialposition (Variables|Default|GetInitialPosition))
  (if (Variables|Default|GetIsForthMovement)
    (LocalVariables|SetTargetLocation _initialposition)
    (else
      (LocalVariables|SetTargetLocation Destination)))
  (Transformation|SetActorLocation Actor (Math|Interpolation|VInterptoConstant (Transformation|GetActorLocation Actor) (LocalVariables|GetTargetLocation) DeltaTime InterpSpeed) false false)
  (Transformation|SetActorRotation Actor (Math|Rotator|FindLookatRotation _initialposition Destination))
  (if (Math|Vector|VectorIsNearlyZero (- (Transformation|GetActorLocation Actor) Destination) 0.0005)
    (Variables|Default|SetIsMovementOver true)))

(fn Stop
  (Variables|Default|SetIsForthMovement true))