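; Nest actor that spawns turtles at its own transform and sends each one toward a destination point.
; BeginPlay calls SpawnTurtle, then binds a handler to OnTurtleSpawned.
; The handler spawns the configured turtle class with a splash sound.
; Movement is delegated to the turtle's components implementing BP_MovementStrategy through an interface message carrying the destination and the turtle's speed.
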(event Custom|OnTurtleSpawned_Event_0
  (bind _returnvalue (Game|SpawnActorfromClass (Variables|Default|GetTurtleToSpawn) (Transformation|GetActorTransform self) "Undefined" 0 0))
  (Audio|PlaySoundatLocation "/Game/Sounds/mixkit-sea-water-splash-1198.mixkit-sea-water-splash-1198" (Transformation|GetActorLocation self) "0, 0, 0" 0.5 1.0 0.0 0 0 0)
  (Class|BPMovementStrategy|MovetoDestination(Message) (Class|Actor|GetComponentsbyInterface _returnvalue "/Game/Blueprints/BP_MovementStrategy.BP_MovementStrategy_C") _returnvalue (Variables|Default|GetDestinationPoint) (Variables|/Script/MovingTurtles.Turtle|GetSpeed _returnvalue)))

(event EventBeginPlay
  (Class|Nest|SpawnTurtle)
  (EventDispatchers|BindEventtoOnTurtleSpawned (delegate Custom|OnTurtleSpawned_Event_0)))

(event Collision|EventActorBeginOverlap
  (params (OtherActor :type Actor%20Object%20Reference)))

(event EventTick
  (params (DeltaSeconds :type Float%20%28single-precision%29)))

(fn ConstructionScript)